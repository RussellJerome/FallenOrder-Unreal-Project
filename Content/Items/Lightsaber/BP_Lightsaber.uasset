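; BP_Lightsaber is the lightsaber item Blueprint, declared here as a skeleton with empty events and functions.
; Its stubs cover blade extension, color, lights, swipes, marks, deflect and reflect effects, throw and catch, and hilt visibility.
; It also exposes Force pull, push, slow, telekinesis and crush hooks.
; No logic is wired: queries return false, zero or nothing, and every other body is empty.
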(event Custom|OnForcePullEnterHold)

(event Custom|OnForceTelekinesisStart
  (params (Instigator :type Actor%20Object%20Reference) (AbilityStateTransitionedFrom :type ERsAbilityState%20Enum :default "None_AbilityState") (AbilityLevel :type ESwAbilityUpgradeLevel%20Enum :default "Level")))

(event Custom|OnForceSlowRenewed
  (params (Instigator :type Actor%20Object%20Reference) (Duration :type Float%20%28single-precision%29) (TimeDilation :type Float%20%28single-precision%29) (AbilityLevel :type ESwAbilityUpgradeLevel%20Enum :default "Level")))

(event Custom|OnForceTelekinesisEnd)

(event Custom|OnForceSlowOverriden
  (params (Instigator :type Actor%20Object%20Reference) (AbilityStateTransitionedFrom :type ERsAbilityState%20Enum :default "None_AbilityState") (AbilityLevel :type ESwAbilityUpgradeLevel%20Enum :default "Level")))

(event Custom|OnForceTelekinesisOverriden
  (params (Instigator :type Actor%20Object%20Reference) (AbilityStateTransitionedFrom :type ERsAbilityState%20Enum :default "None_AbilityState") (AbilityLevel :type ESwAbilityUpgradeLevel%20Enum :default "Level")))

(event Custom|OnForcePullStart
  (params (Instigator :type Actor%20Object%20Reference) (PullDuration :type Float%20%28single-precision%29) (OriginalPullDirection :type Vector) (AbilityStateTransitionedFrom :type ERsAbilityState%20Enum :default "None_AbilityState") (AbilityLevel :type ESwAbilityUpgradeLevel%20Enum :default "Level")))

(event Custom|OnForcePushEnd)

(event Custom|OnForcePullOverriden
  (params (Instigator :type Actor%20Object%20Reference) (AbilityStateTransitionedFrom :type ERsAbilityState%20Enum :default "None_AbilityState") (AbilityLevel :type ESwAbilityUpgradeLevel%20Enum :default "Level")))

(event Custom|OnThrowReturned)

(event Custom|OnForcePushStart
  (params (Instigator :type Actor%20Object%20Reference) (PushVector :type Vector) (PushHitType :type ESwForcePushHitType%20Enum :default "FPHT_Glancing") (OriginalDirection :type Vector) (AbilityStateTransitionedFrom :type ERsAbilityState%20Enum :default "None_AbilityState") (AbilityLevel :type ESwAbilityUpgradeLevel%20Enum :default "Level")))

(event Custom|OnForceSlowEnd)

(event Custom|OnForcePushOverriden
  (params (Instigator :type Actor%20Object%20Reference) (AbilityStateTransitionedFrom :type ERsAbilityState%20Enum :default "None_AbilityState") (AbilityLevel :type ESwAbilityUpgradeLevel%20Enum :default "Level")))

(event Custom|OnForceSlowStart
  (params (Instigator :type Actor%20Object%20Reference) (Duration :type Float%20%28single-precision%29) (TimeDilation :type Float%20%28single-precision%29) (AbilityStateTransitionedFrom :type ERsAbilityState%20Enum :default "None_AbilityState") (AbilityLevel :type ESwAbilityUpgradeLevel%20Enum :default "Level")))

(event EventBeginPlay)

(event Collision|EventActorBeginOverlap
  (params (OtherActor :type Actor%20Object%20Reference)))

(event EventTick
  (params (DeltaSeconds :type Float%20%28single-precision%29)))

(fn ConstructionScript)

(fn CanbeForcePulledbyCharacter
  (params (PullingCharacter :type Rs%20Character%20Object%20Reference))
  (return false))

(fn IsBladeExtended
  (return false))

(fn GetBladeState
  (return ""))

(fn TelekinesisLift
  ;[1 1 1] Maybe
  (return false 0))

(fn IsTelekinesisObject
  (return false 0))

(fn IsForceSlowdownObject
  (return false))

(fn ForceCrushGrab
  (return false))

(fn ChangeLightsaberColor
  (params (New_Blade_Color :type Linear%20Color%20Structure) (New_Blade_Glow_Color :type Linear%20Color%20Structure)))

(fn UpdateControlStack)

(fn LightsaberSFX
  (params (enable :type Boolean)))

(fn FlashLightFadeFinishedFunc)

(fn FlashLightFadeUpdateFunc)

(fn CatchLightsaber
  (params (CatchingCharacter :type Rs%20Character%20Object%20Reference)))

(fn OverchargeEffect
  (params (bStart :type Boolean) (bActivate :type Boolean)))

(fn TelekinesisPush
  (params (Velocity :type Vector)))

(fn TelekinesisDrop
  (params (Velocity :type Vector)))

(fn TelekinesisToss
  (params (Velocity :type Vector)))

(fn ForcePullStart
  (params (pullTime :type Float%20%28single-precision%29) (PullHandLoc :type Vector) (pullHandFwdVector :type Vector)))

(fn ForceSlowdown
  (params (defaultSlowdownLength :type Float%20%28single-precision%29)))

(fn EndForceSlowdown)

(fn ForceCrushRelease)

(fn ForcePullJiggle
  (params (delayWindow :type Float%20%28single-precision%29)))

(fn ForcePullTick
  (params (PullHandLoc :type Vector) (pullHandFwdVector :type Vector) (Progress :type Float%20%28single-precision%29)))

(fn DetachLightsaberfromActor)

(fn ClearDroppedState)

(fn OnForcePullEnd)

(fn LightsaberReflectFX
  (params (ProjectileFX :type Sw%20Projectile%20FX%20Structure)))

(fn LightsaberDeflectFX
  (params (ProjectileFX :type Sw%20Projectile%20FX%20Structure)))

(fn LightsaberThrow)

(fn SetLightsaberMarksState
  (params (bEnabled :type Boolean)))

(fn ExtendRetractBlade
  (params (bExtend :type Boolean) (bInstant :type Boolean)))

(fn UpdateBladeLength
  (params (Delta_Time :type Float%20%28single-precision%29)))

(fn UpdateLights)

(fn LightsaberSwipe
  (params (Delta_Time :type Float%20%28single-precision%29)))

(fn UpdateBlade)

(fn LVLSetHiltVisible
  (params (bNewVisibility :type Boolean)))